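; Player controller for an RTS-style camera and unit selection in a day and wave based game.
; BeginPlay creates the HUD widget, shows the cursor and starts the game state's day and wave counters.
; Clicks select by cursor trace, while drags take BP_HUDMode's hovered actors.
; Input drives BP_CameraPawn with zoom-scaled movement, spring-arm zoom and gated panning that suspends movement; screen-edge scrolling exists but is disconnected.
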(event EventBeginPlay
  (|CallParentFunction)
  (Utilities|FlowControl|Sequence
    (:then_0
      ;[1 1 1] Instantiate all HUDs
      (Input|SetInputModeGameandUI self 0 "LockAlways" false)
      (Utilities|CreateHuds)
      (UserInterface|Viewport|AddtoViewport (Variables|Default|GetDayWaveRef) 0))
    (:then_1
      ;[1 1 1] Instantiate variables for which day and wave to start at
      (bind _asday_night_cycle_game_state (Utilities|Casting|CastToDayNightCycleGameState (Game|GetGameState)))
      (Class|DayNightCycleGameState|InstantiateVariables _asday_night_cycle_game_state 1))
    (:then_2
      (Variables|Default|SetbShowMouseCursor true))))

(event EventTick
  (params (DeltaSeconds :type Float%20%28single-precision%29))
  (bind (_locationx _locationy) (Game|Player|GetMousePosition))
  ;[1 1 1] Handles mouse input for selection
  (if (Variables|Default|GetbIsSelecting)
    (bind _output_get (Variables|Default|SetMouseSelectionDrag (Math|Vector2D|MakeVector2D _locationx _locationy)))
    ;[1 1 1] Set dragging to true if we want to select more than one actor
    (if (and (Math|Vector|NotEqual(Vector) _output_get (stale Input|MouseEvents|LeftMouseButton _output_get) 1.0) (not (Variables|Default|GetIsDragging)))
      (Variables|Default|SetIsDragging true))))

(event Input|ActionEvents|InputActionPan
  (params (Key :type Key%20Structure :default "AnyKey"))
  (bind _output_get (CallFunction|GetCameraPawn))
  (bind _returnvalue (Transformation|GetActorRotation _output_get))
  (bind (_roll _pitch _yaw) (Math|Rotator|BreakRotator _returnvalue))
  ;[1 1 1] Pan Y
  (:Pressed
    (Variables|Default|SetbDisableCamNav true)
    (Utilities|FlowControl|Gate true) ; enters at Open
  )
  (:Released
    (Variables|Default|SetbDisableCamNav false)
    (Utilities|FlowControl|Gate true) ; enters at Close
  ))

(event Input|ActionEvents|InputActionPan
  (params (Key :type Key%20Structure :default "AnyKey"))
  (bind _output_get (CallFunction|GetCameraPawn))
  (bind _returnvalue (Transformation|GetActorRotation _output_get))
  (bind (_roll _pitch _yaw) (Math|Rotator|BreakRotator _returnvalue))
  ;[1 1 1] Pan X (With mouse scroll)
  (:Pressed
    (Variables|Default|SetbDisableCamNav true)
    (Utilities|FlowControl|Gate true) ; enters at Open
  )
  (:Released
    (Variables|Default|SetbDisableCamNav false)
    (Utilities|FlowControl|Gate true) ; enters at Close
  ))

(event Input|ActionEvents|InputActionPan
  (params (Key :type Key%20Structure :default "AnyKey"))
  (bind _output_get (CallFunction|GetCameraPawn))
  (bind _returnvalue (Transformation|GetActorRotation _output_get))
  (bind (_roll _pitch _yaw) (Math|Rotator|BreakRotator _returnvalue))
  ;[1 1 1] Pan X (With Q/E)
  (:Pressed
    (Variables|Default|SetbDisableCamNav true)
    (Utilities|FlowControl|Gate true) ; enters at Open
  )
  (:Released
    (Variables|Default|SetbDisableCamNav false)
    (Utilities|FlowControl|Gate true) ; enters at Close
  ))

(event Input|ActionEvents|InputActionZoomIn
  (params (Key :type Key%20Structure :default "AnyKey"))
  (bind _output_get (CallFunction|GetCameraPawn))
  (bind _springarm (Variables|/Game/Blueprints/BP_CameraPawn.BP_CameraPawn_C|GetSpringArm _output_get))
  ;[1 1 1] Zoom In
  (:Pressed
    (Variables|/Script/Engine.SpringArmComponent|SetTargetArmLength _springarm (Math|Float|Clamp(Float) (- (Variables|/Script/Engine.SpringArmComponent|GetTargetArmLength _springarm) (Variables|Default|GetZoomSensitivity)) (Variables|Default|GetMinArmDistance) (Variables|Default|GetMaxArmDistance)))))

(event Input|ActionEvents|InputActionZoomOut
  (params (Key :type Key%20Structure :default "AnyKey"))
  (bind _output_get (CallFunction|GetCameraPawn))
  (bind _springarm (Variables|/Game/Blueprints/BP_CameraPawn.BP_CameraPawn_C|GetSpringArm _output_get))
  ;[1 1 1] Zoom Out
  (:Pressed
    (Variables|/Script/Engine.SpringArmComponent|SetTargetArmLength _springarm (Math|Float|Clamp(Float) (+ (Variables|Default|GetZoomSensitivity) (Variables|/Script/Engine.SpringArmComponent|GetTargetArmLength _springarm)) (Variables|Default|GetMinArmDistance) (Variables|Default|GetMaxArmDistance)))))

(event Input|AxisEvents|InputAxisRotate
  (params (AxisValue :type Float%20%28single-precision%29))
  (bind _output_get (CallFunction|GetCameraPawn))
  (bind _returnvalue (Transformation|GetActorRotation _output_get))
  (bind (_roll _pitch _yaw) (Math|Rotator|BreakRotator _returnvalue))
  ;[1 1 1] Pan X (With Q/E)
  (Utilities|FlowControl|Gate true
    (:Exit
      (Transformation|SetActorRotation (CallFunction|GetCameraPawn) (Math|Rotator|MakeRotator _roll _pitch (+ _yaw AxisValue))))))

(event Input|AxisEvents|InputAxisMoveRight
  (params (AxisValue :type Float%20%28single-precision%29))
  (bind _output_get (CallFunction|GetCameraPawn))
  (bind _movesensitivity (CallFunction|MovementSpeedCalculation))
  (bind _fastmovemultiplier (Variables|Default|GetFastMoveMultiplier))
  (bind _transform (Utilities|MovementY AxisValue _movesensitivity _fastmovemultiplier _output_get))
  (bind (_location _rotation _scale) (Math|Transform|BreakTransform _transform))
  (bind (_x _y) (Math|Vector|BreakVector _location))
  ;[1 1 1] Movement Y
  (if (not (Variables|Default|GetbDisableCamNav))
    (Transformation|SetActorTransform _output_get (Math|Transform|MakeTransform (Math|Vector|MakeVector _x _y 1e+02) _rotation _scale))))

(event Input|AxisEvents|InputAxisMoveForward
  (params (AxisValue :type Float%20%28single-precision%29))
  (bind _camerapawnref (Variables|References|GetCameraPawnRef))
  ;[1 1 1] Movement X
  (if (not (Variables|Default|GetbDisableCamNav))
    (Transformation|SetActorTransform _camerapawnref (Utilities|MovementX (CallFunction|MovementSpeedCalculation) (Variables|Default|GetFastMoveMultiplier) AxisValue _camerapawnref))))

(event Input|MouseEvents|MouseX
  (params (AxisValue :type Float%20%28single-precision%29))
  (bind _output_get (CallFunction|GetCameraPawn))
  (bind _returnvalue (Transformation|GetActorRotation _output_get))
  (bind (_roll _pitch _yaw) (Math|Rotator|BreakRotator _returnvalue))
  ;[1 1 1] Pan X (With mouse scroll)
  (Utilities|FlowControl|Gate true
    (:Exit
      (Transformation|SetActorRotation (CallFunction|GetCameraPawn) (Math|Rotator|MakeRotator _roll _pitch (+ _yaw (* (Variables|Default|GetPanSensitivity) AxisValue)))))))

(event Input|MouseEvents|MouseY
  (params (AxisValue :type Float%20%28single-precision%29))
  (bind _output_get (CallFunction|GetCameraPawn))
  (bind _returnvalue (Transformation|GetActorRotation _output_get))
  (bind (_roll _pitch _yaw) (Math|Rotator|BreakRotator _returnvalue))
  ;[1 1 1] Pan Y
  (Utilities|FlowControl|Gate true
    (:Exit
      (Transformation|SetActorRotation (CallFunction|GetCameraPawn) (Math|Rotator|MakeRotator _roll (Math|Float|Clamp(Float) (+ _pitch (* (Variables|Default|GetPanSensitivity) AxisValue)) -15.0 45.0) _yaw)))))

(event Input|MouseEvents|MouseX
  (params (AxisValue :type Float%20%28single-precision%29))
  ;[1 1 1] Edge Movement
)

(event Input|MouseEvents|MouseY
  (params (AxisValue :type Float%20%28single-precision%29))
  ;[1 1 1] Edge Movement
)

(event Input|MouseEvents|LeftMouseButton
  (params (Key :type Key%20Structure :default "AnyKey"))
  (bind _hitresult (Game|Player|GetHitResultUnderCursorbyChannel "TraceTypeQuery3" true))
  (bind (_locationx _locationy) (Game|Player|GetMousePosition))
  (bind (_locationx_2 _locationy_2) (Game|Player|GetMousePosition))
  (bind _hitactor (Collision|BreakHitResult _hitresult))
  ;[1 1 1] Handles mouse input for selection
  (:Pressed
    (Variables|Default|SetbIsSelecting true)
    (bind _output_get (Variables|Default|SetMouseSelectionStart (Math|Vector2D|MakeVector2D _locationx _locationy))))
  (:Released
    (Variables|Default|SetbIsSelecting false)
    (Variables|Default|SetMouseSelectionEnd (Math|Vector2D|MakeVector2D _locationx_2 _locationy_2))
    (if (Variables|Default|GetIsDragging)
      ;[1 1 1] Get selected actors
      (bind _asbp_hudmode (Utilities|Casting|CastToBP_HUDMode (HUD|GetHUD)))
      (Variables|Default|SetSelectedActors (Variables|/Game/Modes/BP_HUDMode.BP_HUDMode_C|GetHovered%20Actors _asbp_hudmode))
      (Development|PrintString (Utilities|String|BuildString(Integer) "" "Selected: " (Utilities|Array|Length (Variables|/Game/Modes/BP_HUDMode.BP_HUDMode_C|GetHovered%20Actors _asbp_hudmode))))
      (Variables|Default|SetIsDragging false)
      (else
        ;[1 1 1] If only one actor is selected
        (Variables|Default|SetSelectedActors (Utilities|Array|MakeArray _hitactor))
        (Development|PrintString (Utilities|String|Append "Selected: " (Utilities|GetDisplayName _hitactor)))))))

(fn ConstructionScript)

(fn GetCameraPawn
  (Utilities|IsValid (Variables|References|GetCameraPawnRef)
    (:Is%20Valid
      _)
    (:Is%20Not%20Valid
      (bind _asbp_camera_pawn (Utilities|Casting|CastToBP_CameraPawn (Pawn|GetControlledPawn)))
      (bind _output_get (Variables|References|SetCameraPawnRef _asbp_camera_pawn))))
  (return _output_get))

(fn MovementSpeedCalculation
  (return (Math|Float|Clamp(Float) (/ (Variables|/Script/Engine.SpringArmComponent|GetTargetArmLength (Variables|/Game/Blueprints/BP_CameraPawn.BP_CameraPawn_C|GetSpringArm (CallFunction|GetCameraPawn))) 1e+02) 5.0 2e+01)))