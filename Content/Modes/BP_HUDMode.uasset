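; BP_HUDMode is a HUD that detects which units or buildings fall inside the player's drag-selection rectangle.
; On BeginPlay it caches the BP_SkrymtPlayerController, whose drag state and start and drag mouse points define the rectangle.
; Each DrawHUD during a drag fills HoveredActors with units in the rectangle, or with buildings if no units are found, and prints the count.
; When no drag is active, HoveredActors is emptied.
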(event EventBeginPlay
  (bind _asbp_skrymt_player_controller (Utilities|Casting|CastToBP_SkrymtPlayerController (Game|Player|GetOwningPlayerController)))
  (Variables|Default|SetPlayerController _asbp_skrymt_player_controller))

(event EventDrawHUD
  (params (SizeX :type Integer) (SizeY :type Integer))
  (bind _playercontroller (Variables|Default|GetPlayerController))
  (bind _mouseselectionstart (Variables|/Game/Modes/BP_SkrymtPlayerController.BP_SkrymtPlayerController_C|GetMouseSelectionStart _playercontroller))
  (bind _mouseselectiondrag (Variables|/Game/Modes/BP_SkrymtPlayerController.BP_SkrymtPlayerController_C|GetMouseSelectionDrag _playercontroller))
  (bind _outactors (Class|HUD|GetActorsinSelectionRectangle "/Game/Blueprints/BP_Unit.BP_Unit_C" _mouseselectionstart _mouseselectiondrag true false))
  (bind _outactors_2 (Class|HUD|GetActorsinSelectionRectangle "/Game/Blueprints/BP_Building.BP_Building_C" _mouseselectionstart _mouseselectiondrag true false))
  (bind _returnvalue (Utilities|Array|Length _outactors))
  (bind _returnvalue_2 (> _returnvalue 0))
  (if (Variables|/Game/Modes/BP_SkrymtPlayerController.BP_SkrymtPlayerController_C|GetIsDragging _playercontroller)
    (Development|PrintString (Utilities|String|BuildString(Integer) "" "Hovered: " (Math|Integer|SelectInt _returnvalue (Utilities|Array|Length _outactors_2) _returnvalue_2)))
    (if _returnvalue_2
      (Variables|Default|SetHovered%20Actors _outactors)
      (else
        (Variables|Default|SetHovered%20Actors _outactors_2)))
    (else
      (Utilities|Array|Resize (Variables|Default|GetHovered%20Actors) 0))))

(fn ConstructionScript)